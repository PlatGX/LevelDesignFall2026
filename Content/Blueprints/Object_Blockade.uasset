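; Blockade actor that appears as a burning obstacle of logs when its trigger box is first overlapped.
; A one-shot overlap calls SpawnObject, which spawns fire, smoke and explosion emitters at three billboard markers, starts fire audio, plays a 2D explosion sound and makes three log components visible.
; The player reference cached on BeginPlay is not used as a filter, so any overlapping actor can trigger it.
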(event `self.ReceiveBeginPlay`
  ;[1 0.6634 0.7857] Casting spawner to Player
  (bind _asbp_third_person_character (cast `/Game/ThirdPerson/Blueprints/BP_ThirdPersonCharacter` (`GameplayStatics.GetPlayerCharacter` 0)))
  (set `self.As BP Third Person Character` _asbp_third_person_character))

(event `self.Box.OnComponentBeginOverlap`
  (params (OverlappedComponent :type "PrimitiveComponent Object Reference") (OtherActor :type "Actor Object Reference") (OtherComp :type "PrimitiveComponent Object Reference") (OtherBodyIndex :type Integer) (bFromSweep :type Boolean) (SweepResult :type "HitResult Structure (by ref)"))
  ;[1 0.6634 0.7857] Casting spawner to Player
  (if true
    (`/Engine/EditorBlueprintResources/StandardMacros.DoOnce` false
      (:`Completed`
        (`self.SpawnObject`)))))

(event `SpawnObject`
  (bind _billboard (`self.Billboard`))
  (bind _billboard1 (`self.Billboard1`))
  (bind _billboard2 (`self.Billboard2`))
  ;[0.466 0.8171 1] Object Spawning
  (`|ExecutionSequence`
    (:`then_0`
      (`GameplayStatics.SpawnEmitterAtLocation` "/Game/M5VFXVOL2/Particles/Reference/Fireloop/4_bigfire_pt.4_bigfire_pt" (`SceneComponent.K2_GetComponentLocation` _billboard) (`SceneComponent.K2_GetComponentRotation` _billboard) (4.0 4.0 4.0))
      (`AudioComponent.Play` (`self.FireSource`) 0.0))
    (:`then_1`
      (`GameplayStatics.SpawnEmitterAtLocation` "/Game/M5VFXVOL2/Particles/Reference/Smoke/5_6_smoke6_pt2.5_6_smoke6_pt2" (`SceneComponent.K2_GetComponentLocation` _billboard1) (`SceneComponent.K2_GetComponentRotation` _billboard1) (4.0 4.0 4.0)))
    (:`then_2`
      (`GameplayStatics.SpawnEmitterAtLocation` "/Game/StarterContent/Particles/P_Explosion.P_Explosion" (`SceneComponent.K2_GetComponentLocation` _billboard2) (`SceneComponent.K2_GetComponentRotation` _billboard2) (4.0 4.0 4.0))
      (`GameplayStatics.SpawnSound2D` "/Game/StarterContent/Audio/Explosion02.Explosion02" 1.0 1.0 0.0 null))
    (:`then_3`
      (`SceneComponent.SetVisibility` (`self.Log`) true false)
      (`SceneComponent.SetVisibility` (`self.Log1`) true false)
      (`SceneComponent.SetVisibility` (`self.Log2`) true false))))

(fn `UserConstructionScript`)