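; AI spawner actor with a trigger box that spawns a group of three different AI types the first time it is overlapped.
; A DoOnce gate calls SpawnObject, which spawns BP_AI, BP_AI2 and BP_AI3 at separate Billboard transforms, playing the spawn sound with each.
; BeginPlay caches the player character, but the overlap comparison against it is unwired, so any overlapping actor triggers the spawn.
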(event `self.ReceiveBeginPlay`
  ;[1 0.6634 0.7857] Casting spawner to Player
  (bind _asbp_third_person_character (cast `/Game/ThirdPerson/Blueprints/BP_ThirdPersonCharacter` (`GameplayStatics.GetPlayerCharacter` 0)))
  (set `self.As BP Third Person Character` _asbp_third_person_character))

(event `self.Box.OnComponentBeginOverlap`
  (params (OverlappedComponent :type "PrimitiveComponent Object Reference") (OtherActor :type "Actor Object Reference") (OtherComp :type "PrimitiveComponent Object Reference") (OtherBodyIndex :type Integer) (bFromSweep :type Boolean) (SweepResult :type "HitResult Structure (by ref)"))
  ;[1 0.6634 0.7857] Casting spawner to Player
  (if true
    (`/Engine/EditorBlueprintResources/StandardMacros.DoOnce` false
      (:`Completed`
        (`self.SpawnObject`)))))

(event `SpawnObject`
  (bind _billboard (`self.Billboard`))
  (bind _billboard1 (`self.Billboard1`))
  (bind _billboard2 (`self.Billboard2`))
  ;[0.466 0.8171 1] Object Spawning
  (`|ExecutionSequence`
    (:`then_0`
      (`|SpawnActorFromClass` "/Game/ThirdPerson/Blueprints/BP_AI2.BP_AI2_C" (`KismetMathLibrary.MakeTransform` (`SceneComponent.K2_GetComponentLocation` _billboard) (`SceneComponent.K2_GetComponentRotation` _billboard)) "Undefined" "MultiplyWithRoot" null null)
      (`AudioComponent.Play` (`self.SpawnSound`) 0.0))
    (:`then_1`
      (`|SpawnActorFromClass` "/Game/ThirdPerson/Blueprints/BP_AI3.BP_AI3_C" (`KismetMathLibrary.MakeTransform` (`SceneComponent.K2_GetComponentLocation` _billboard1) (`SceneComponent.K2_GetComponentRotation` _billboard1)) "Undefined" "MultiplyWithRoot" null null)
      (`AudioComponent.Play` (`self.SpawnSound`) 0.0))
    (:`then_2`
      (`|SpawnActorFromClass` "/Game/ThirdPerson/Blueprints/BP_AI.BP_AI_C" (`KismetMathLibrary.MakeTransform` (`SceneComponent.K2_GetComponentLocation` _billboard2) (`SceneComponent.K2_GetComponentRotation` _billboard2)) "Undefined" "MultiplyWithRoot" null null)
      (`AudioComponent.Play` (`self.SpawnSound`) 0.0))))

(fn `UserConstructionScript`)