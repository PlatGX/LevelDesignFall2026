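; An interactable actor that lets the player switch on smoke and fire effects with the E key.
; It creates a prompt widget on BeginPlay and shows or hides it as the player character enters or leaves the trigger.
; Any overlap enables input and nothing disables it, so E keeps working after leaving.
; Pressing E makes both particle components visible and plays FireSource from the start.
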(event `self.ReceiveBeginPlay`
  ;[0.9949 0.6783 1] Getting Player Input
  (bind _returnvalue (`|CreateWidget` "/Game/Blueprints/Particle_Text.Particle_Text_C" (`GameplayStatics.GetPlayerController` 0)))
  (set `self.Particle_Interact` _returnvalue))

(event `self.Particle_Trigger.OnComponentBeginOverlap`
  (params (OverlappedComponent :type "PrimitiveComponent Object Reference") (OtherActor :type "Actor Object Reference") (OtherComp :type "PrimitiveComponent Object Reference") (OtherBodyIndex :type Integer) (bFromSweep :type Boolean) (SweepResult :type "HitResult Structure (by ref)"))
  ;[0.8424 1 0.98] Particle Trigger Event
  (`self.EnableInput` (`GameplayStatics.GetPlayerController` 0))
  (if (== OtherActor (`GameplayStatics.GetPlayerCharacter` 0))
    (`UserWidget.AddToViewport` (`self.Particle_Interact`) 0)))

(event `self.Particle_Trigger.OnComponentEndOverlap`
  (params (OverlappedComponent :type "PrimitiveComponent Object Reference") (OtherActor :type "Actor Object Reference") (OtherComp :type "PrimitiveComponent Object Reference") (OtherBodyIndex :type Integer))
  ;[0.8424 1 0.98] Particle Trigger Event
  (if (== (`GameplayStatics.GetPlayerCharacter` 0) OtherActor)
    (`Widget.RemoveFromParent` (`self.Particle_Interact`))))

(event `Key|E`
  (params (Key :type "Key Structure"))
  ;[1 1 1] Getting Key Input
  (:`Pressed`
    (`SceneComponent.SetVisibility` (`self.SmokeParticles`) true false)
    (`SceneComponent.SetVisibility` (`self.FireParticles`) true false)
    (`AudioComponent.Play` (`self.FireSource`) 0.0)))

(fn `UserConstructionScript`)