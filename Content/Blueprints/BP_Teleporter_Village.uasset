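; Village teleporter actor that opens the lvl_Start level when anything overlaps its teleport trigger.
; Overlapping the button trigger enables input, and for the player also shows an interact widget and plays the Invalid_Action sound.
; Pressing E reveals the lightning and galactic fields and the trigger, changing only visibility.
; Leaving removes the widget but leaves input enabled.
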(event `Key|E`
  (params (Key :type "Key Structure"))
  ;[1 0.6979 0.6979] Key Interaction
  (:`Pressed`
    (`SceneComponent.SetVisibility` (`self.N_LightningField`) true false)
    (`SceneComponent.SetVisibility` (`self.N_GalacticField`) true false)
    (`SceneComponent.SetVisibility` (`self.Teleport_Trigger`) true false)))

(event `self.Teleport_Trigger.OnComponentBeginOverlap`
  (params (OverlappedComponent :type "PrimitiveComponent Object Reference") (OtherActor :type "Actor Object Reference") (OtherComp :type "PrimitiveComponent Object Reference") (OtherBodyIndex :type Integer) (bFromSweep :type Boolean) (SweepResult :type "HitResult Structure (by ref)"))
  ;[1 0.575 0.9573] Teleport Trigger
  (`GameplayStatics.OpenLevel` "lvl_Start"))

(event `self.ReceiveBeginPlay`
  ;[0.8909 1 0.4991] Widget Reference
  (bind _returnvalue (`|CreateWidget` "/Game/Blueprints/Widget_Interact.Widget_Interact_C" (`GameplayStatics.GetPlayerController` 0)))
  (set `self.Interact_Widget` _returnvalue))

(event `self.Button_Tigger.OnComponentBeginOverlap`
  (params (OverlappedComponent :type "PrimitiveComponent Object Reference") (OtherActor :type "Actor Object Reference") (OtherComp :type "PrimitiveComponent Object Reference") (OtherBodyIndex :type Integer) (bFromSweep :type Boolean) (SweepResult :type "HitResult Structure (by ref)"))
  ;[0.7322 0.9398 1] Widget Trigger
  (`self.EnableInput` (`GameplayStatics.GetPlayerController` 0))
  (if (== OtherActor (`GameplayStatics.GetPlayerCharacter` 0))
    (`UserWidget.AddToViewport` (`self.Interact_Widget`) 0)
    (`GameplayStatics.PlaySound2D` "/Engine/VREditor/Sounds/UI/Invalid_Action.Invalid_Action" 1.0 1.0 0.0 null null)))

(event `self.Button_Tigger.OnComponentEndOverlap`
  (params (OverlappedComponent :type "PrimitiveComponent Object Reference") (OtherActor :type "Actor Object Reference") (OtherComp :type "PrimitiveComponent Object Reference") (OtherBodyIndex :type Integer))
  ;[0.7322 0.9398 1] Widget Trigger
  (if (== (`GameplayStatics.GetPlayerCharacter` 0) OtherActor)
    (`Widget.RemoveFromParent` (`self.Interact_Widget`))))

(fn `UserConstructionScript`)